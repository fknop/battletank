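; Tank component that aims the turret and barrel at a world location, fires projectiles and tracks ammo.
; AimAt solves a toss velocity for the launch speed, feeds pitch and yaw deltas to barrel and turret, and switches between Aiming and Locked by alignment.
; Fire spawns and launches a projectile from the barrel socket in either state.
; Firing decrements ammo, then delays through Reloading or sets OutOfAmmo.
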(event Custom|Fired_Event
  (bind _result (Math|Integer|DecrementInt (Variables|Default|GetAmmo))
    (:%20%20
      (if (<= _result 0)
        (Variables|Default|SetFiringState "NewEnumerator4")
        (else
          (Variables|Default|SetFiringState "NewEnumerator1")
          (Utilities|FlowControl|Delay (Variables|Default|GetReloadingTime))
          (Variables|Default|SetFiringState "NewEnumerator0"))))))

(event Custom|Aimed_Event
  (switch Utilities|FlowControl|Switch|SwitchonFiringStatus (Variables|Default|GetFiringState)
    (:NewEnumerator0
      _)
    (:NewEnumerator2
      _))
  (Variables|Default|SetFiringState "NewEnumerator0")
  (Utilities|FlowControl|Delay 1.0)
  (switch Utilities|FlowControl|Switch|SwitchonFiringStatus (Variables|Default|GetFiringState)
    (:NewEnumerator0
      (Variables|Default|SetFiringState "NewEnumerator2"))))

(event EventBeginPlay
  (Variables|Default|SetAmmo (Variables|Default|GetInitialAmmo))
  (Utilities|FlowControl|Delay (Variables|Default|GetReloadingTime))
  (Variables|Default|SetFiringState "NewEnumerator0"))

(fn Aimat
  (params (Location :type Vector%20%28by%20ref%29))
  (bind _barrel (Variables|Default|GetBarrel))
  (Utilities|IsValid _barrel
    (:Is%20Valid
      (bind (_tossvelocity _returnvalue) (Class|GameplayStatics|BlueprintSuggestProjectileVelocity (Transformation|GetSocketLocation _barrel "Projectile") Location (Variables|Default|GetLaunchSpeed) 0.0 "DoNotTrace" 0.0 false false))
      (if _returnvalue
        ;[1 1 1] Move the turret and barrel
        (Utilities|FlowControl|Sequence
          (:then_0
            (switch Utilities|FlowControl|Switch|SwitchonFiringStatus (Variables|Default|GetFiringState)
              (:NewEnumerator0
                _)
              (:NewEnumerator2
                _))
            (if (Math|Vector|Equal(Vector) (Math|Vector|Normalize _tossvelocity) (Math|Vector|Normalize (Math|Vector|GetForwardVector (Variables|Default|GetBarrel))) 0.05)
              (Variables|Default|SetFiringState "NewEnumerator2")
              (else
                (Variables|Default|SetFiringState "NewEnumerator0"))))
          (:then_1
            (CallFunction|MoveBarrel (Math|Vector|Normalize _tossvelocity))
            (CallFunction|MoveTurret (Math|Vector|Normalize _tossvelocity))))))))

(fn MoveBarrel
  (params (AimDirection :type Vector%20%28by%20ref%29))
  (Default|Elevate (Variables|Default|GetBarrel) (.Pitch (Math|Rotator|BreakRotator (Math|Rotator|Delta(Rotator) (Math|Rotator|MakeRotationfromAxes AimDirection "0, 0, 0" "0, 0, 0") (Math|Rotator|MakeRotationfromAxes (Math|Vector|GetForwardVector (Variables|Default|GetBarrel)) "0, 0, 0" "0, 0, 0"))))))

(fn MoveTurret
  (params (AimDirection :type Vector%20%28by%20ref%29))
  (Default|Rotate (Variables|Default|GetTurret) (.Yaw (Math|Rotator|BreakRotator (Math|Rotator|Delta(Rotator) (Math|Rotator|MakeRotationfromAxes AimDirection "0, 0, 0" "0, 0, 0") (Math|Rotator|MakeRotationfromAxes (Math|Vector|GetForwardVector (Variables|Default|GetTurret)) "0, 0, 0" "0, 0, 0"))))))

(fn Initialize
  (params (Turret :type Tank%20Turret%20BP%20Object%20Reference%20%28by%20ref%29) (Barrel :type Tank%20Barrel%20BP%20Object%20Reference%20%28by%20ref%29))
  (Variables|Default|SetTurret Turret)
  (Variables|Default|SetBarrel Barrel))

(fn Fire
  (bind _returnvalue (Utilities|Name|MakeLiteralName "Projectile"))
  (bind _barrel (Variables|Default|GetBarrel))
  (switch Utilities|FlowControl|Switch|SwitchonFiringStatus (Variables|Default|GetFiringState)
    (:NewEnumerator0
      _)
    (:NewEnumerator2
      _))
  (bind _returnvalue_2 (Game|SpawnActorfromClass (Variables|Default|GetProjectileBlueprint) (Math|Transform|MakeTransform (Transformation|GetSocketLocation _barrel _returnvalue) (Transformation|GetSocketRotation _barrel _returnvalue) "1.000000,1.000000,1.000000") "AdjustIfPossibleButAlwaysSpawn" 0 0))
  (Default|LaunchProjectile _returnvalue_2 (Variables|Default|GetLaunchSpeed))
  (CallFunction|FiredEvent))

(fn GetFiringState
  (return (Variables|Default|GetFiringState)))

(fn GetRemainingAmmo
  (return (Variables|Default|GetAmmo)))