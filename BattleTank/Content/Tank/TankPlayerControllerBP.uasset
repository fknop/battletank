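; Player controller Blueprint for the tank game that sets up the player's UI when play begins.
; BeginPlay runs the parent logic, then InitUI creates the PlayerUI widget and adds it to the viewport.
; It also prints a debug message naming the possessed tank, obtained through GetControlledTank.
; Tick only forwards to the parent, and the construction script is empty.
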(event EventBeginPlay
  (|CallParentFunction)
  (CallFunction|InitUI)
  (Development|PrintString (Utilities|String|ToString(Text) (Utilities|Text|FormatText "Posessing: {Name}" (Utilities|Text|ToText(Object) (CallFunction|GetControlledTank)))) true true "(R=0.000000,G=0.660000,B=1.000000,A=1.000000)" 2e+01))

(event EventTick
  (params (DeltaSeconds :type Float%20%28single-precision%29))
  (|CallParentFunction DeltaSeconds))

(fn ConstructionScript)

(fn InitUI
  (bind _returnvalue (UserInterface|CreateWidget "/Game/UI/PlayerUI.PlayerUI_C"))
  (UserInterface|Viewport|AddtoViewport _returnvalue 0))