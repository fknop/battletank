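; Movement component for a tank that turns forward and turn intentions into left and right track throttle.
; Initialize stores both tracks; forward throw drives them equally and turn throw drives them in opposite directions.
; RequestDirectMove translates AI path velocity into throws via dot and cross products with the forward vector.
; Both intents set throttle directly, so the turn call overwrites the forward one.
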(event EventBeginPlay)

(event EventTick
  (params (DeltaSeconds :type Float%20%28single-precision%29)))

(event EventOnRequestDirectMove
  (params (MoveVelocity :type Vector%20%28by%20ref%29) (bForceMaxSpeed :type Boolean))
  (bind _returnvalue (Math|Vector|Normalize MoveVelocity))
  (bind _returnvalue_2 (Components|GetOwner))
  (bind _returnvalue_3 (Transformation|GetActorForwardVector _returnvalue_2))
  (bind _returnvalue_4 (Math|Vector|Normalize _returnvalue_3))
  (Input|IntendMoveForward (Math|Vector|DotProduct _returnvalue _returnvalue_4))
  (Input|IntendTurnRight (.Z (Math|Vector|BreakVector (Math|Vector|CrossProduct _returnvalue_4 _returnvalue)))))

(fn IntendMoveForward
  (params (Throw :type Float%20%28single-precision%29))
  (Default|SetThrottle (Variables|Default|GetLeft%20Track) Throw)
  (Default|SetThrottle (Variables|Default|GetRight%20Track) Throw))

(fn Initialize
  (params (Left%20Track :type Tank%20Track%20BP%20Object%20Reference%20%28by%20ref%29) (Right%20Track :type Tank%20Track%20BP%20Object%20Reference%20%28by%20ref%29))
  (Variables|Default|SetLeft%20Track Left%20Track)
  (Variables|Default|SetRight%20Track Right%20Track))

(fn IntendTurnRight
  (params (Throw :type Float%20%28single-precision%29))
  (Default|SetThrottle (Variables|Default|GetLeft%20Track) Throw)
  (Default|SetThrottle (Variables|Default|GetRight%20Track) (* Throw -1.0)))