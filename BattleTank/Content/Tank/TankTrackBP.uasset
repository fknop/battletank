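; Tank track component that propels its owning tank through physics forces on the owner's root primitive.
; SetThrottle accumulates clamped input, which each component hit consumes and resets, so drive only applies while the track is in contact.
; On hit, DriveTrack pushes forward at the track's location.
; A halved, mass-scaled counter-force, computed from the track's sideways velocity over delta time, then cancels lateral slip.
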(event Custom|OnComponentHit_Event
  (params (HitComponent :type Primitive%20Component%20Object%20Reference) (OtherActor :type Actor%20Object%20Reference) (OtherComp :type Primitive%20Component%20Object%20Reference) (NormalImpulse :type Vector) (Hit :type Hit%20Result%20Structure%20%28by%20ref%29))
  (CallFunction|OnHit))

(event EventBeginPlay
  (EventDispatchers|AssignOnComponentHit (delegate Custom|OnComponentHit_Event)))

(fn DriveTrack
  (bind _asprimitive_component (Utilities|Casting|CastToPrimitiveComponent (VehicleSound|GetRootComponent (Components|GetOwner))))
  (Class|PrimitiveComponent|AddForceatLocation _asprimitive_component (* (* (Math|Vector|GetForwardVector) (Variables|Default|GetCurrentThrottle)) (Variables|Default|GetTrackMaxDrivingForce)) (Transformation|GetWorldLocation) "None"))

(fn OnHit
  (bind _returnvalue (Components|GetOwner))
  (bind _returnvalue_2 (Transformation|GetActorRightVector _returnvalue))
  (CallFunction|DriveTrack)
  ;[1 1 1] Correction force
  (bind _asprimitive_component (Utilities|Casting|CastToPrimitiveComponent (VehicleSound|GetRootComponent (Components|GetOwner))))
  (Physics|AddForce _asprimitive_component (/ (* (* _returnvalue_2 (/ (* (Math|Vector|DotProduct _returnvalue_2 (Transformation|GetComponentVelocity)) -1.0) (Utilities|Time|GetWorldDeltaSeconds))) (Physics|GetMass _asprimitive_component)) 2.0) "None" false)
  (Variables|Default|SetCurrentThrottle 0.0))

(fn SetThrottle
  (params (Throttle :type Float%20%28single-precision%29))
  (Variables|Default|SetCurrentThrottle (Math|Float|Clamp(Float) (+ Throttle (Variables|Default|GetCurrentThrottle)) -1.0)))