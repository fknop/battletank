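; Tank aiming component that points a tank's turret and barrel so a projectile fired at a given launch speed reaches a target location.
; AimAt solves the toss velocity from the barrel's Projectile socket with SuggestProjectileVelocity, without tracing, and acts only when a solution exists.
; MoveBarrel passes the pitch difference to the barrel's Elevate, and MoveTurret passes the yaw difference to the turret's Rotate.
; Barrel and turret references are supplied through setter functions.
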(event EventBeginPlay)

(fn Aimat
  (params (Location :type Vector%20%28by%20ref%29) (LaunchSpeed :type Float%20%28single-precision%29))
  (bind _barrel (Variables|Default|GetBarrel))
  (Utilities|IsValid _barrel
    (:Is%20Valid
      (bind (_tossvelocity _returnvalue) (Class|GameplayStatics|BlueprintSuggestProjectileVelocity (Transformation|GetSocketLocation _barrel "Projectile") Location LaunchSpeed 0.0 "DoNotTrace" 0.0 false false))
      (if _returnvalue
        (CallFunction|MoveBarrel (Math|Vector|Normalize _tossvelocity))
        (CallFunction|MoveTurret (Math|Vector|Normalize _tossvelocity))))))

(fn SetBarrel
  (params (Barrel :type Tank%20Barrel%20BP%20Object%20Reference%20%28by%20ref%29))
  (Variables|Default|SetBarrel Barrel))

(fn MoveBarrel
  (params (AimDirection :type Vector%20%28by%20ref%29))
  (Default|Elevate (Variables|Default|GetBarrel) (.Pitch (Math|Rotator|BreakRotator (Math|Rotator|Delta(Rotator) (Math|Rotator|MakeRotationfromAxes AimDirection "0, 0, 0" "0, 0, 0") (Math|Rotator|MakeRotationfromAxes (Math|Vector|GetForwardVector (Variables|Default|GetBarrel)) "0, 0, 0" "0, 0, 0"))))))

(fn SetTurret
  (params (Turret :type Tank%20Turret%20BP%20Object%20Reference%20%28by%20ref%29))
  (Variables|Default|SetTurret Turret))

(fn MoveTurret
  (params (AimDirection :type Vector%20%28by%20ref%29))
  (Default|Rotate (Variables|Default|GetTurret) (.Yaw (Math|Rotator|BreakRotator (Math|Rotator|Delta(Rotator) (Math|Rotator|MakeRotationfromAxes AimDirection "0, 0, 0" "0, 0, 0") (Math|Rotator|MakeRotationfromAxes (Math|Vector|GetForwardVector (Variables|Default|GetTurret)) "0, 0, 0" "0, 0, 0"))))))