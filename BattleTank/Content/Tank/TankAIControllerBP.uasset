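; AI controller for enemy tanks that tracks and shoots at the first player's tank.
; Each Tick, while that tank is valid, it aims the controlled TankBP at the player's location and fires whenever CanFire allows, with no range or sight check.
; A Delay of the tank's ReloadingTime re-arms CanFire after each shot.
; Helper functions wrap the casts for both tanks and an unused player controller lookup.
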(event EventTick
  (params (DeltaSeconds :type Float%20%28single-precision%29))
  (bind _tank (CallFunction|GetControlledTank))
  (bind _tank_2 (CallFunction|GetPlayerTank))
  (|CallParentFunction DeltaSeconds)
  (Utilities|IsValid _tank_2
    (:Is%20Valid
      (Default|Aimat _tank (Transformation|GetActorLocation _tank_2))
      (if (Variables|Default|GetCanFire)
        (Variables|Default|SetCanFire false)
        (Default|Fire _tank)
        (Utilities|FlowControl|Delay (Variables|/Game/Tank/TankBP.TankBP_C|GetReloadingTime _tank))
        (Variables|Default|SetCanFire true)))))

(fn ConstructionScript)

(fn GetControlledTank
  (bind _astank_bp (Utilities|Casting|CastToTankBP (Pawn|GetControlledPawn)))
  (return _astank_bp))

(fn GetPlayerTank
  (params (PlayerIndex :type Integer))
  (bind _astank_bp (Utilities|Casting|CastToTankBP (Game|Player|GetPlayerPawn PlayerIndex)))
  (return _astank_bp))

(fn GetTankPlayerController
  (params (PlayerIndex :type Integer))
  (bind _astank_player_controller_base_bp (Utilities|Casting|CastToTankPlayerControllerBaseBP (Game|GetPlayerController PlayerIndex)))
  (return _astank_player_controller_base_bp))