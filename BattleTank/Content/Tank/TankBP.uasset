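; Tank pawn Blueprint that handles camera aiming, driving and firing through input bindings.
; Azimuth gimbal and spring arm rotate with aim input, while AimAt forwards target locations to TankAimingComponent, which receives barrel and turret at construction.
; Movement intent goes through TankMovementComponent, initialized with both tracks, alongside direct per-track throttle inputs.
; Firing spawns a projectile at the barrel socket and launches it, gated by a reload delay.
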(event Collision|EventActorBeginOverlap
  (params (OtherActor :type Actor%20Object%20Reference)))

(event EventTick
  (params (DeltaSeconds :type Float%20%28single-precision%29)))

(event Input|ActionEvents|InputActionFire
  (params (Key :type Key%20Structure :default "AnyKey"))
  ;[1 1 1] Fire Input binding
  (:Pressed
    (if (Variables|Firing|GetCanFire)
      (Variables|Firing|SetCanFire false)
      (CallFunction|Fire)
      (Utilities|FlowControl|Delay (Variables|Firing|GetReloadingTime))
      (Variables|Firing|SetCanFire true))))

(event Input|AxisEvents|InputAxisLeftTrackThrottle
  (params (AxisValue :type Float%20%28single-precision%29))
  ;[1 1 1] Throttle Input Binding (keyboard only)
  (Default|SetThrottle (Variables|Default|GetLeft%20Track) AxisValue))

(event Input|AxisEvents|InputAxisRightTrackThrottle
  (params (AxisValue :type Float%20%28single-precision%29))
  ;[1 1 1] Throttle Input Binding (keyboard only)
  (Default|SetThrottle (Variables|Default|GetRight%20Track) AxisValue))

(event Input|AxisEvents|InputAxisAimAzimuth
  (params (AxisValue :type Float%20%28single-precision%29))
  ;[1 1 1] Aiming input binding
  (Transformation|AddLocalRotation (Variables|Default|GetAzimuth%20Gimbal) (Math|Rotator|MakeRotator 0.0 0.0 (* AxisValue (Utilities|Time|GetWorldDeltaSeconds) 1e+02)) false false))

(event Input|AxisEvents|InputAxisMoveFoward
  (params (AxisValue :type Float%20%28single-precision%29))
  ;[1 1 1] Fly-By-Wire Input Binding
  (Default|IntendMoveForward (Variables|Default|GetTankMovementComponent) AxisValue))

(event Input|AxisEvents|InputAxisMoveBackward
  (params (AxisValue :type Float%20%28single-precision%29))
  ;[1 1 1] Fly-By-Wire Input Binding
  (Default|IntendMoveForward (Variables|Default|GetTankMovementComponent) AxisValue))

(event Input|AxisEvents|InputAxisAimElevation
  (params (AxisValue :type Float%20%28single-precision%29))
  ;[1 1 1] Aiming input binding
  (Transformation|AddLocalRotation (Variables|Default|GetSpringArm) (Math|Rotator|MakeRotator 0.0 (* AxisValue (Utilities|Time|GetWorldDeltaSeconds) 1e+02) 0.0) false false))

(fn ConstructionScript
  (CallFunction|SetBarrelReference)
  (CallFunction|SetTurretReference)
  (Default|Initialize (Variables|Default|GetTankMovementComponent) (Variables|Default|GetLeft%20Track) (Variables|Default|GetRight%20Track)))

(fn Aimat
  (params (Location :type Vector%20%28by%20ref%29))
  (Default|Aimat (Variables|Default|GetTankAimingComponent) Location (Variables|Firing|GetLaunchSpeed)))

(fn SetBarrelReference
  (Default|SetBarrel (Variables|Default|GetTankAimingComponent) (Variables|Default|GetBarrel)))

(fn SetTurretReference
  (Default|SetTurret (Variables|Default|GetTankAimingComponent) (Variables|Default|GetTurret)))

(fn Fire
  (bind _returnvalue (Utilities|Name|MakeLiteralName "Projectile"))
  (bind _barrel (Variables|Default|GetBarrel))
  (bind _returnvalue_2 (Game|SpawnActorfromClass (Variables|Setup|GetProjectileBlueprint) (Math|Transform|MakeTransform (Transformation|GetSocketLocation _barrel _returnvalue) (Transformation|GetSocketRotation _barrel _returnvalue) "1.000000,1.000000,1.000000") "AdjustIfPossibleButAlwaysSpawn" 0 0))
  (Default|LaunchProjectile _returnvalue_2 (Variables|Firing|GetLaunchSpeed)))