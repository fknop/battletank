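; Base player controller for a tank that aims the controlled tank at whatever lies under the on-screen crosshair and switches to spectating when the tank dies.
; Each tick it deprojects the crosshair's viewport-relative position, line-traces from the camera on the Camera channel up to a maximum range, and passes any hit to the pawn's aiming component.
; On begin play it caches that component and binds to the tank's death event.
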(event Custom|OnDeath_Event
  (CallFunction|OnDeath))

(event EventBeginPlay
  (|CallParentFunction)
  (Variables|Default|SetAimingComponent (Actor|GetComponentbyClass (Pawn|GetControlledPawn) "/Game/Components/TankAimingComponentBP.TankAimingComponentBP_C"))
  (bind _astank_bp (Utilities|Casting|CastToTankBP (Pawn|GetControlledPawn)))
  (EventDispatchers|AssignOnDeath _astank_bp (delegate Custom|OnDeath_Event)))

(event EventTick
  (params (DeltaSeconds :type Float%20%28single-precision%29))
  (|CallParentFunction DeltaSeconds)
  (CallFunction|AimTowardsCrosshair))

(fn ConstructionScript)

(fn AimTowardsCrosshair
  (bind (_hit_location _return_value) (CallFunction|GetSightRayHitLocation))
  (Utilities|IsValid (Pawn|GetControlledPawn)
    (:Is%20Valid
      (if _return_value
        (Default|Aimat (Variables|Default|GetAimingComponent) _hit_location)))))

(fn GetSightRayHitLocation
  (bind (_look_direction _return_value) (CallFunction|GetLookDirection))
  (bind (_hitlocation _return_value_2) (CallFunction|GetLookHitLocation _look_direction))
  (if _return_value
    ;[1 1 1] Here, Ben Tristem always return true, resetting the barrel when out of landscape
    (return _hitlocation _return_value_2)
    (else
      (return "0, 0, 0" false))))

(fn CrosshairScreenLocation
  (bind _returnvalue (Viewport|GetViewportSize))
  (bind (_x _y) (Math|Vector2D|BreakVector2D _returnvalue))
  (return (Math|Vector2D|MakeVector2D (* (Variables|Default|GetCrossHairXLocation) _x) (* _y (Variables|Default|GetCrossHairYLocation)))))

(fn GetLookDirection
  (bind _location (CallFunction|CrosshairScreenLocation))
  (bind _returnvalue (Game|GetPlayerController 0))
  (bind (_worldposition _worlddirection _returnvalue_2) (Class|GameplayStatics|DeprojectScreentoWorld _returnvalue _location))
  (return _worlddirection _returnvalue_2))

(fn GetLookHitLocation
  (params (LookDirection :type Vector%20%28by%20ref%29))
  (bind _returnvalue (Game|GetPlayerCameraManager 0))
  (bind _returnvalue_2 (Camera|GetCameraLocation _returnvalue))
  (bind (_outhit _returnvalue_3) (Collision|LineTraceByChannel _returnvalue_2 (+ _returnvalue_2 (* LookDirection (Variables|Default|GetMaximumRange))) "TraceTypeQuery2" false 0 "None"))
  (if _returnvalue_3
    (return (.Location (Collision|BreakHitResult _outhit)) true)
    (else
      (return "0, 0, 0" false))))

(fn OnDeath
  (Class|BasePlayerController|StartSpectatingOnly))