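; Tank track component that drives its owning tank and counters sideways slippage.
; SetThrottle pushes the owner's root primitive along the track's forward vector at the track's location, scaled by throttle and maximum driving force.
; Each tick it measures velocity along the owner's right vector and applies half the mass-scaled force needed to cancel it, presumably splitting the correction between two tracks.
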(event EventBeginPlay)

(event EventTick
  (params (DeltaSeconds :type Float%20%28single-precision%29))
  (bind _returnvalue (Components|GetOwner))
  (bind _returnvalue_2 (Transformation|GetActorRightVector _returnvalue))
  ;[1 1 1] Correction force
  (bind _asprimitive_component (Utilities|Casting|CastToPrimitiveComponent (VehicleSound|GetRootComponent (Components|GetOwner))))
  (Physics|AddForce _asprimitive_component (/ (* (* _returnvalue_2 (/ (* (Math|Vector|DotProduct _returnvalue_2 (Transformation|GetComponentVelocity)) -1.0) DeltaSeconds)) (Physics|GetMass _asprimitive_component)) 2.0) "None" false))

(fn SetThrottle
  (params (Throttle :type Float%20%28single-precision%29))
  (bind _asprimitive_component (Utilities|Casting|CastToPrimitiveComponent (VehicleSound|GetRootComponent (Components|GetOwner))))
  (Class|PrimitiveComponent|AddForceatLocation _asprimitive_component (* (* (Math|Vector|GetForwardVector) Throttle) (Variables|Default|GetTrackMaxDrivingForce)) (Transformation|GetWorldLocation) "None"))