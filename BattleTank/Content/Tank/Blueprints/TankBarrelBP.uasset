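; Tank barrel component that pitches itself up and down to set the gun's elevation.
; Elevate clamps a relative speed input to -1 to 1, scales it by max degrees per second and frame delta time, and adds it to the current pitch.
; The result is clamped between elevation limits and applied as relative rotation with zero roll and yaw.
; BeginPlay and Tick are unused, so movement happens only when Elevate is called.
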(event EventBeginPlay)

(event EventTick
  (params (DeltaSeconds :type Float%20%28single-precision%29)))

(fn Elevate
  (params (RelativeSpeed :type Float%20%28single-precision%29))
  (Transformation|SetRelativeRotation (Math|Rotator|MakeRotator 0.0 (Math|Float|Clamp(Float) (+ (* (Math|Float|Clamp(Float) RelativeSpeed -1.0) (Variables|Setup|GetMaxDegreesPerSecond) (Utilities|Time|GetWorldDeltaSeconds)) (.Pitch (Math|Rotator|BreakRotator (Variables|Default|GetRelativeRotation)))) (Variables|Setup|GetMinElevationDegrees) (Variables|Setup|GetMaxElevationDegrees)) 0.0) false false))